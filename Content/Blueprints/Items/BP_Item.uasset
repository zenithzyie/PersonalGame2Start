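; BP_Item is an item that can be picked up, dropped and used.
; PickUp attaches it to the given parent at the right-hand item socket and turns off the Cube's physics and collision.
; DropItem detaches the Cube in world space and restores physics and collision.
; UsePrimary, intended for left-click use while held, is a stub that only prints, as the other events also do for debugging.
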(event `PickUp`
  (params (Parent :type "SceneComponent Object Reference"))
  (bind _cube (`self.Cube`))
  (`KismetSystemLibrary.PrintString` "PickUpItem")
  (`self.K2_AttachToComponent` Parent "item_socket_r" "SnapToTarget" "SnapToTarget" "KeepRelative")
  (`PrimitiveComponent.SetSimulatePhysics` _cube false) ; Stop Simulating
  (`PrimitiveComponent.SetCollisionEnabled` _cube "NoCollision"))

(event `DropItem`
  (bind _cube (`self.Cube`))
  (`KismetSystemLibrary.PrintString` "DropItem")
  (`SceneComponent.K2_DetachFromComponent` _cube "KeepWorld" "KeepWorld" "KeepRelative" true)
  (`PrimitiveComponent.SetSimulatePhysics` _cube true) ; Start Simulating
  (`PrimitiveComponent.SetCollisionEnabled` _cube "QueryAndPhysics"))

(event `UsePrimary`
  (params (Char :type "/Game/ThirdPerson/Blueprints/BP_ThirdPersonCharacter Object Reference"))
  (`KismetSystemLibrary.PrintString` "UsePrimary"))

(fn `UserConstructionScript`)