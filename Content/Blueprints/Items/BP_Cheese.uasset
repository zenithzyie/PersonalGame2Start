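; BP_Cheese is a pickup item that gives the using character the cheese.
; BeginPlay creates an interact prompt widget and a "got cheese" widget, though only the latter is displayed in this graph.
; UsePrimary sets HasTheCheese on the character, prints a debug string, shows the pickup widget and hides the cube mesh.
; After a short delay, it removes the widget and destroys the actor.
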(event `self.ReceiveBeginPlay`
  (`|ExecutionSequence`
    (:`then_0`
      (bind _returnvalue (`|GenericCreateObject` "/Game/Blueprints/P_Interact.P_Interact_C"))
      (set `self.CreateInteractPrompt` _returnvalue))
    (:`then_1`
      (bind _returnvalue_2 (`|GenericCreateObject` "/Game/Blueprints/P_GetCheese.P_GetCheese_C"))
      (set `self.GotCheese` _returnvalue_2))))

(event `self.UsePrimary`
  (params (Char :type "/Game/ThirdPerson/Blueprints/BP_ThirdPersonCharacter Object Reference"))
  (bind _gotcheese (`self.GotCheese`))
  (set `/Game/ThirdPerson/Blueprints/BP_ThirdPersonCharacter.HasTheCheese` true Char)
  (`KismetSystemLibrary.PrintString` "HASCHEESE")
  (`UserWidget.AddToViewport` _gotcheese 0)
  (`SceneComponent.SetVisibility` (`self.Cube`) false false)
  (`KismetSystemLibrary.Delay` 3.0)
  (`Widget.RemoveFromParent` _gotcheese)
  (`self.K2_DestroyActor`))

(fn `UserConstructionScript`
  (`parent.UserConstructionScript`))