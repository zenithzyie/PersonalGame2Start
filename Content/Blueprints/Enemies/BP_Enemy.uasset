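; BP_Enemy is an enemy actor that prints a threatening greeting on BeginPlay.
; It defines a TakeDamage event, but nothing is wired to it.
; Disconnected logic would subtract damage from Health, print the new value, and destroy the actor once the CheckIfAlive helper finds Health no longer above zero.
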(event `self.ReceiveBeginPlay`
  (`KismetSystemLibrary.PrintString` "Hello. I have been programmed to destroy you."))

(event `TakeDamage`
  (params (Bye :type "Float (double-precision)" :default 0.2)))

(fn `CheckIfAlive`
  (params (Health :type "Float (double-precision)"))
  (returns (IsAlive :type Boolean))
  (return (> Health 0.0)))

(fn `UserConstructionScript`)